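; AirgustBase is a wind gust actor that flies forward, grows and expires after a maximum lifetime.
; Initialize stores the speed, sets the life span and creates a dynamic instance of the wind noise material.
; Each tick lerps current scale toward MaxSize, moves with a sweep by Speed per frame, unscaled by delta time, and counts the material's Lifetime parameter down from one.
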(event `Initialize`
  (params (Speed :type "Float (double-precision)"))
  (set `self.Speed` Speed)
  (`self.SetLifeSpan` (`self.MaxLifetime`))
  (bind _returnvalue (`PrimitiveComponent.CreateDynamicMaterialInstance` (`self.Windgust_Windgust_Base`) 0 "/Game/Materials/M_WindNoise_Inst.M_WindNoise_Inst" "None"))
  (set `self.Material` _returnvalue))

(event `self.ReceiveTick`
  (params (DeltaSeconds :type "Float (single-precision)"))
  (set `self.CurrentTimeAlive` (+ DeltaSeconds (`self.CurrentTimeAlive`)))
  (`|ExecutionSequence`
    (:`then_0`
      (`self.SetActorRelativeScale3D` (`KismetMathLibrary.VLerp` (`self.GetActorRelativeScale3D`) (`self.MaxSize`) (/ (`self.CurrentTimeAlive`) (`self.GrowTime`)))))
    (:`then_1`
      (`self.K2_SetActorLocation` (+ (`self.K2_GetActorLocation`) (* (`self.GetActorForwardVector`) (`self.Speed`))) true))
    (:`then_2`
      (`MaterialInstanceDynamic.SetScalarParameterValue` (`self.Material`) "Lifetime" (- 1.0 (/ (`self.CurrentTimeAlive`) (`self.MaxLifetime`)))))))

(fn `UserConstructionScript`)