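; Airgust projectile that flies forward and knocks physics-capable actors other than the player character into a ragdoll.
; Initialize sets speed, scales lifespan by its ratio to max speed and creates a dynamic wind material.
; Tick sweeps the actor forward and lowers the material's Lifetime parameter over time.
; Sphere overlaps send ragdoll and speed-scaled, slightly upward impulse messages through BPI_Physics, gated by a DoOnce with delayed reset.
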(event `Initialize`
  (params (Owner :type "/Game/Blueprints/BP_BaseCharacter Object Reference") (Speed :type "Float (double-precision)") (MaxSpeed :type "Float (double-precision)"))
  (set `self.Player` Owner)
  (bind _output_get (set `self.Speed` Speed))
  (`self.SetLifeSpan` (+ (* (/ _output_get MaxSpeed) (`self.MaxLifetime`)) 0.1))
  (bind _returnvalue (`PrimitiveComponent.CreateDynamicMaterialInstance` (`self.Windgust_Windgust_Head`) 0 "/Game/Materials/M_WindNoise_Inst.M_WindNoise_Inst" "None"))
  (set `self.Material` _returnvalue))

(event `self.ReceiveTick`
  (params (DeltaSeconds :type "Float (single-precision)"))
  (bind (_returnvalue_location _returnvalue_rotation _returnvalue_scale) (`KismetMathLibrary.BreakTransform` (`self.GetTransform`)))
  (set `self.CurrentTimeAlive` (+ DeltaSeconds (`self.CurrentTimeAlive`)))
  (`self.K2_SetActorTransform` (`KismetMathLibrary.MakeTransform` (+ (`self.K2_GetActorLocation`) (* (`self.GetActorForwardVector`) (`self.Speed`))) _returnvalue_rotation _returnvalue_scale) true)
  (`MaterialInstanceDynamic.SetScalarParameterValue` (`self.Material`) "Lifetime" (- 1.0 (/ (`self.CurrentTimeAlive`) (`self.MaxLifetime`)))))

(event `self.SphereTrigger.OnComponentBeginOverlap`
  (params (OverlappedComponent :type "PrimitiveComponent Object Reference") (OtherActor :type "Actor Object Reference") (OtherComp :type "PrimitiveComponent Object Reference") (OtherBodyIndex :type Integer) (bFromSweep :type Boolean) (SweepResult :type "HitResult Structure (by ref)"))
  (if (and (`KismetSystemLibrary.DoesImplementInterface` OtherActor "/Game/Blueprints/Interfaces/BPI_Physics.BPI_Physics_C") (!= (`GameplayStatics.GetObjectClass` OtherActor) "/Game/Blueprints/PlayerCharacter/BP_PlayerCharacter.BP_PlayerCharacter_C") (> (`self.Speed`) 0.0))
    (`self.CharacterForceEffect` OtherActor)))

(event `CharacterForceEffect`
  (params (Actor :type "Actor Object Reference"))
  (`/Engine/EditorBlueprintResources/StandardMacros.DoOnce` false :!label _label
    (:`Completed`
      (message `/Game/Blueprints/Interfaces/BPI_Physics.ToggleRagdoll` Actor true 3.0)
      (message `/Game/Blueprints/Interfaces/BPI_Physics.ForceImpulseMovement` Actor (* (+ (* (`self.GetActorUpVector`) 0.2) (`self.GetActorForwardVector`)) (* (+ (`self.Speed`) 1.0) 1000.0)))
      (`KismetSystemLibrary.Delay` 3.0)
      (goto _label :!via `Reset`))))

(fn `UserConstructionScript`)