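; Spawner actor that creates AI enemies of a requested type at its own transform.
; SpawnEnemy maps the enemy type to a Villager or Musket Hunter pawn class and behavior tree, spawns it ignoring collision, then initializes it.
; It binds each enemy's death event and reports spawns and deaths to the third-person game mode's enemy count, cached on BeginPlay.
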(event `self.ReceiveBeginPlay`
  (bind _asbp_third_person_game_mode (cast `/Game/Blueprints/BP_ThirdPersonGameMode` (`GameplayStatics.GetGameMode`)))
  (set `self.Gamemode` _asbp_third_person_game_mode))

(event `SpawnEnemy`
  (params (`Enemy Type` :type "/Game/Blueprints/AI/Enum_EnemyType Enum" :default "NewEnumerator0"))
  (bind (_returnvalue_location _returnvalue_rotation) (`KismetMathLibrary.BreakTransform` (`self.GetTransform`)))
  (bind (_pawnclass _behaviortree) (`self.SwitchEnemyTypes` `Enemy Type`))
  (bind _returnvalue (`AIBlueprintHelperLibrary.SpawnAIFromClass` _pawnclass _behaviortree _returnvalue_location _returnvalue_rotation true null))
  (bind _asbp_base_enemy (cast `/Game/Blueprints/AI/BP_BaseEnemy` _returnvalue))
  (`/Game/Blueprints/AI/BP_BaseEnemy.Initialize` _asbp_base_enemy)
  (add `/Game/Blueprints/BP_BaseCharacter.OnDeath` _asbp_base_enemy (delegate `OnEnemyDeath`))
  (`/Game/Blueprints/BP_ThirdPersonGameMode.ChangeEnemyAmount` (`self.Gamemode`) 1))

(event `OnEnemyDeath`
  (`/Game/Blueprints/BP_ThirdPersonGameMode.ChangeEnemyAmount` (`self.Gamemode`) -1))

(fn `SwitchEnemyTypes`
  (params (EnemyType :type "/Game/Blueprints/AI/Enum_EnemyType Enum" :default "NewEnumerator0"))
  (returns (PawnClass :type "Pawn Class Reference") (BehaviorTree :type "BehaviorTree Object Reference"))
  (switch `/Game/Blueprints/AI/Enum_EnemyType` EnemyType
    (:`NewEnumerator0`
      (return "/Game/Blueprints/AI/Villager/BP_Villager.BP_Villager_C" "/Game/Blueprints/AI/Villager/BT_Villager.BT_Villager"))
    (:`NewEnumerator1`
      (return "/Game/Blueprints/AI/MusketHunter/BP_MusketHunter.BP_MusketHunter_C" "/Game/Blueprints/AI/MusketHunter/BT_MusketHunter.BT_MusketHunter"))))

(fn `UserConstructionScript`)