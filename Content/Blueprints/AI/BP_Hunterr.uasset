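; BP_Hunterr is an AI character that takes damage, heals and dies.
; On BeginPlay it casts its mesh's ABP_Manny and its BP_AIController, then hands the behavior tree and anim blueprint to the controller through SetupAIC.
; Damage lowers CurrentHealth and triggers Death at zero, which only sets the IsDead blackboard key.
; Healing clamps health between zero and MaxHealth.
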(event `self.ReceiveBeginPlay`
  (bind _asabp_manny (cast `/Game/Characters/Mannequins/Animations/ABP_Manny` (`SkeletalMeshComponent.GetAnimInstance` (`self.Mesh`))))
  (set `self.AnimBP` _asabp_manny)
  (bind _asbp_aicontroller (cast `/Game/Blueprints/AI/BP_AIController` (`AIBlueprintHelperLibrary.GetAIController` self)))
  (bind _output_get (set `self.AIController` _asbp_aicontroller))
  (`/Game/Blueprints/AI/BP_AIController.SetupAIC` _output_get (`self.BehaviorTree`) (`self.AnimBP`)))

(event `self.TakeDamage`
  (params (DamageAmount :type "Float (double-precision)"))
  (bind _output_get (set `self.CurrentHealth` (- (`self.CurrentHealth`) DamageAmount)))
  (if (<= _output_get 0.0)
    (`self.Death`)))

(event `self.Heal`
  (params (HealAmount :type "Float (double-precision)"))
  (set `self.CurrentHealth` (`KismetMathLibrary.FClamp` (+ (`self.CurrentHealth`) HealAmount) 0.0 (`self.MaxHealth`))))

(event `self.Death`
  (`/Game/Blueprints/AI/FuncLib_AI.SetBB_Bool` (`self.AIController`) "IsDead" true))

(fn `UserConstructionScript`)