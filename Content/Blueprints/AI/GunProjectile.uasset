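; Physics-driven gun projectile that damages BPI_Combat actors, can ricochet once off other surfaces, and expires after a set lifetime.
; Combat hits deal randomly varied damage, play a flesh impact sound, and trace downward to place a blood decal before destroying the projectile.
; Other hits compare velocity with the hit normal to either destroy it or flag a ricochet with sound.
; ForceImpulseMovement deflects the bullet with a doubled impulse.
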(event `self.ReceiveBeginPlay`
  (`self.SetLifeSpan` (`self.MaxLifetime`)))

(event `self.Sphere.OnComponentHit`
  (params (HitComponent :type "PrimitiveComponent Object Reference") (OtherActor :type "Actor Object Reference") (OtherComp :type "PrimitiveComponent Object Reference") (NormalImpulse :type "Vector Structure") (Hit :type "HitResult Structure (by ref)"))
  (if (`KismetSystemLibrary.DoesImplementInterface` OtherActor "/Game/Blueprints/Interfaces/BPI_Combat.BPI_Combat_C")
    (`self.DealDamage` OtherActor)
    (elif (or (> (`KismetMathLibrary.Dot_VectorVector` Hit_Normal (`KismetMathLibrary.Normal` (`SceneComponent.GetComponentVelocity` (`self.Sphere`)))) 0.75) (`self.HasRicocheted`))
      (`self.EnvironmentImpact`)
      (else
        (`self.Ricochet` Hit_Location)))))

(event `DealDamage`
  (params (OtherActor :type "Actor Object Reference"))
  (bind _returnvalue (`self.K2_GetActorLocation` OtherActor))
  (bind _damage (`self.CalculateDamage`))
  (message `/Game/Blueprints/Interfaces/BPI_Combat.TakeDamage` OtherActor _damage (`self.GetInstigator`))
  (message `/Game/Blueprints/Interfaces/BPI_ActorSoundEffects.PlaySoundAtLocation` OtherActor "/Game/Sounds/SFX/Impacts/BulletFleshImpact_Cue.BulletFleshImpact_Cue")
  (bind _outhit (`KismetSystemLibrary.LineTraceSingle` _returnvalue (+ _returnvalue (* (`self.GetActorUpVector` OtherActor) -200.0)) "TraceTypeQuery1"))
  (`GameplayStatics.SpawnDecalAttached` "/Game/Megascans/Decals/High_Velocity_Blood_Spatter_sfjjcfzp/MI_High_Velocity_Blood_Spatter_sfjjcfzp_2K.MI_High_Velocity_Blood_Spatter_sfjjcfzp_2K" (30.0 100.0 100.0) (`.HitComponent` (`GameplayStatics.BreakHitResult` _outhit)) "None" (`.Location` (`GameplayStatics.BreakHitResult` _outhit)) (`KismetMathLibrary.MakeRotFromX` (`KismetMathLibrary.NegateVector` (`.Normal` (`GameplayStatics.BreakHitResult` _outhit)))) "KeepWorldPosition" 20.0)
  (`self.K2_DestroyActor`))

(event `EnvironmentImpact`
  (`self.K2_DestroyActor`))

(event `Ricochet`
  (params (HitLocation :type "Vector Structure"))
  (`GameplayStatics.PlaySoundAtLocation` "/Game/Sounds/SFX/Gun/WallRicochet_Cue.WallRicochet_Cue" HitLocation (struct) 1.0 1.0 0.0 null null null null)
  (set `self.HasRicocheted` true))

(event `/Game/Blueprints/Interfaces/BPI_Physics.ForceImpulseMovement`
  (params (Impulse :type "Vector Structure"))
  (`PrimitiveComponent.AddImpulse` (`self.Sphere`) (* Impulse 2.0) "None" false)
  (`KismetSystemLibrary.PrintString` "Bullet Deflected"))

(fn `CalculateDamage`
  (returns (Damage :type "Float (double-precision)"))
  (return (`/Game/Blueprints/FL_Misc.RandomVarianceFloat` (`self.BaseDamage`) (`self.DamageVariance`))))

(fn `UserConstructionScript`)