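; BP_BaseEnemy is the base AI enemy character, linking its Manny animation Blueprint and AI controller to a behavior tree.
; On BeginPlay it caches both references and passes the behavior tree and anim instance to the controller's SetupAIC.
; On death it runs the parent handler, sends a kill message to the attacker, and sets the IsDead blackboard key.
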(event `self.ReceiveBeginPlay`
  (bind _asabp_manny (cast `/Game/Characters/Mannequins/Animations/ABP_Manny` (`SkeletalMeshComponent.GetAnimInstance` (`self.Mesh`))))
  (set `self.AnimBP` _asabp_manny)
  (bind _asbp_aicontroller (cast `/Game/Blueprints/AI/BP_AIController` (`AIBlueprintHelperLibrary.GetAIController` self)))
  (bind _output_get (set `self.AIController` _asbp_aicontroller))
  (`/Game/Blueprints/AI/BP_AIController.SetupAIC` _output_get (`self.BehaviorTree`) (`self.AnimBP`)))

(event `/Game/Blueprints/Combat.Death`
  (params (Attacker :type "Actor Object Reference"))
  (`parent.Death` Attacker)
  (message `/Game/Blueprints/Combat.GotKill` Attacker)
  (`/Game/Blueprints/AI/FuncLib_AI.SetBB_Bool` (`self.AIController`) "IsDead" true))

(fn `UserConstructionScript`)