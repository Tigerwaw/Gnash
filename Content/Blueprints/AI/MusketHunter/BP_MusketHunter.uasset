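; BP_MusketHunter is a musket-wielding AI hunter that fires a projectile at a given attack location.
; Its Attack event calls SpawnBullet, which plays gunshot particles and sound just in front of the actor.
; It then spawns a scaled-down GunProjectile there and launches it with a physics impulse along the direction from the hunter to the target, scaled by ProjectileSpeed.
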(event `/Game/Blueprints/Combat.Attack`
  (params (AttackLocation :type "Vector Structure"))
  (`self.SpawnBullet` AttackLocation))

(fn `SpawnBullet`
  (params (Target :type "Vector Structure"))
  (locals (SpawnLocation :type "Vector Structure"))
  (bind _output_get (set `local.SpawnLocation` (+ (`self.K2_GetActorLocation`) (* (`self.GetActorForwardVector`) 50.0))))
  (`NiagaraFunctionLibrary.SpawnSystemAtLocation` "/Game/Particles/PS_Gunshot.PS_Gunshot" _output_get)
  (`GameplayStatics.PlaySoundAtLocation` "/Game/Sounds/SFX/Gun/LoudGunshot_Cue.LoudGunshot_Cue" (`local.SpawnLocation`) (struct) 1.0 1.0 0.0 null null null null)
  (bind _returnvalue (`|SpawnActorFromClass` "/Game/Blueprints/GunProjectile.GunProjectile_C" (`KismetMathLibrary.MakeTransform` (`local.SpawnLocation`) (struct) (0.15 0.15 0.15)) "AlwaysSpawn" "OverrideRootScale" null self))
  (`PrimitiveComponent.AddImpulse` (`/Game/Blueprints/GunProjectile.Sphere` _returnvalue) (* (`KismetMathLibrary.GetDirectionUnitVector` (`self.K2_GetActorLocation`) Target) (`self.ProjectileSpeed`)) "None" false))

(fn `UserConstructionScript`
  (`parent.UserConstructionScript`))