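; Main menu camera path actor that flies the player's BP_CustomSpectator pawn along a spline.
; BeginPlay caches the pawn and moves it to the spline component's location.
; Tick advances distance by Speed, places the pawn there facing a look-ahead point further along the spline, and restarts past the end.
; The actor destroys itself on Tick when no valid spectator exists.
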(event `self.ReceiveBeginPlay`
  (bind _asbp_custom_spectator (cast `/Game/Blueprints/BP_CustomSpectator` (`GameplayStatics.GetPlayerPawn` 0)))
  (bind _output_get (set `self.As BP Custom Spectator` _asbp_custom_spectator))
  (`self.K2_SetActorTransform` _output_get (`KismetMathLibrary.MakeTransform` (`SceneComponent.K2_GetComponentLocation` (`self.Spline`))) false false))

(event `self.ReceiveTick`
  (params (DeltaSeconds :type "Float (single-precision)"))
  (`/Engine/EditorBlueprintResources/StandardMacros.IsValid` (`self.As BP Custom Spectator`)
    (:`Is Valid`
      (set `self.DistanceTravelled` (+ (* DeltaSeconds (`self.Speed`)) (`self.DistanceTravelled`)))
      (`self.UpdateSpectatorPawnLocation`))
    (:`Is Not Valid`
      (`self.K2_DestroyActor`))))

(event `UpdateSpectatorPawnLocation`
  (bind _spline (`self.Spline`))
  (bind _returnvalue_location (`KismetMathLibrary.BreakTransform` (`SplineComponent.GetTransformAtDistanceAlongSpline` _spline (`self.DistanceTravelled`) "World" false)))
  (bind _returnvalue_location_2 (`KismetMathLibrary.BreakTransform` (`SplineComponent.GetTransformAtDistanceAlongSpline` _spline (+ (`self.DistanceTravelled`) 500.0) "World" false)))
  (`self.K2_SetActorTransform` (`self.As BP Custom Spectator`) (`KismetMathLibrary.MakeTransform` _returnvalue_location (`KismetMathLibrary.FindLookAtRotation` _returnvalue_location _returnvalue_location_2)) false false)
  (if (> (`self.DistanceTravelled`) (`SplineComponent.GetSplineLength` (`self.Spline`)))
    (set `self.DistanceTravelled` 0.0)))

(fn `UserConstructionScript`)