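; Base character Blueprint providing shared health, combat, death, ragdoll and noise-making sound logic.
; Damage clamps health, plays blood and sound effects on heavier hits, and triggers death with ragdoll and a timed lifespan.
; Ragdoll toggles mesh physics, then after a delay re-snaps capsule and mesh using the cached spawn transform if still alive.
; AllowDamageCheck filters self, non-BPI_Combat and repeated targets, with a retriggerable-delay event clearing the last target.
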(event `self.ReceiveBeginPlay`
  (set `self.MeshSpawnTransform` (`SceneComponent.GetRelativeTransform` (`self.Mesh`))))

(event `ClearLastAttackedTarget`
  (`KismetSystemLibrary.RetriggerableDelay` 0.5)
  (set `self.LastAttackedTarget` null))

(event `self.TakeDamage`
  (params (DamageAmount :type "Float (double-precision)") (Attacker :type "Actor Object Reference"))
  ;[1 1 1] Combat
  (if (not (`self.IsDead`))
    (`self.CalculateDamage` DamageAmount)
    (`self.OnTakeDamage`)
    (if (<= (`self.CurrentHealth`) 0.0)
      (`self.Death` Attacker))))

(event `self.Heal`
  (params (HealAmount :type "Float (double-precision)"))
  ;[1 1 1] Combat
  (set `self.CurrentHealth` (`KismetMathLibrary.FClamp` (+ (`self.CurrentHealth`) HealAmount) 0.0 (`self.MaxHealth`)))
  (`self.OnHeal`))

(event `self.Death`
  (params (Attacker :type "Actor Object Reference"))
  ;[1 1 1] Combat
  (`self.OnDeath`)
  (`self.ToggleRagdoll` true 20.0)
  (set `self.IsDead` true)
  (`self.SetLifeSpan` 5.0))

(event `self.ChangeMovementSpeed`
  (params (NewSpeed :type "Float (double-precision)"))
  ;[1 1 1] Combat
  (set `CharacterMovementComponent.MaxWalkSpeed` NewSpeed (`self.CharacterMovement`)))

(event `self.GotKill`
  ;[1 1 1] Combat
  (`self.OnKill`))

(event `self.ToggleRagdoll`
  (params (Active :type Boolean) (ResetTime :type "Float (double-precision)"))
  (bind _mesh (`self.Mesh`))
  ;[1 1 1] Ragdoll Physics
  (`CharacterMovementComponent.SetMovementMode` (`self.CharacterMovement`) "MOVE_None" 0)
  (`PrimitiveComponent.SetCollisionEnabled` (`self.CapsuleComponent`) "NoCollision")
  (`PrimitiveComponent.SetCollisionObjectType` _mesh "ECC_PhysicsBody")
  (`PrimitiveComponent.SetCollisionEnabled` _mesh "QueryAndPhysics")
  (`SkeletalMeshComponent.SetAllBodiesSimulatePhysics` _mesh true)
  (set `self.IsRagdolled` true)
  (`KismetSystemLibrary.Delay` ResetTime)
  (`self.ResetRagdoll`))

(event `self.ResetRagdoll`
  (bind _mesh (`self.Mesh`))
  (bind (_meshspawntransform_location _meshspawntransform_rotation) (`KismetMathLibrary.BreakTransform` (`self.MeshSpawnTransform`)))
  (bind _mesh_2 (`self.Mesh`))
  (bind _capsulecomponent (`self.CapsuleComponent`))
  (bind (_returnvalue_x _returnvalue_y _returnvalue_z) (`KismetMathLibrary.BreakVector` (`SceneComponent.K2_GetComponentLocation` _capsulecomponent)))
  (bind (_returnvalue_x_2 _returnvalue_y_2) (`KismetMathLibrary.BreakVector` (`SceneComponent.K2_GetComponentLocation` (`self.Mesh`))))
  ;[1 1 1] Ragdoll Physics
  (if (not (`self.IsDead`))
    (`PrimitiveComponent.SetCollisionEnabled` (`self.CapsuleComponent`) "QueryAndPhysics")
    (`PrimitiveComponent.SetCollisionObjectType` _mesh_2 "ECC_Pawn")
    (`PrimitiveComponent.SetCollisionEnabled` _mesh_2 "QueryAndPhysics")
    (`SkeletalMeshComponent.SetAllBodiesSimulatePhysics` _mesh_2 false)
    (`SceneComponent.K2_SetWorldLocation` _capsulecomponent (`KismetMathLibrary.MakeVector` _returnvalue_x_2 _returnvalue_y_2 _returnvalue_z) false false)
    (`SceneComponent.K2_AttachToComponent` (`self.Mesh`) (`self.CapsuleComponent`) "None" "SnapToTarget" "KeepRelative" "KeepRelative" true)
    (`SceneComponent.K2_SetRelativeLocation` _mesh _meshspawntransform_location false false)
    (`SceneComponent.K2_SetRelativeRotation` _mesh _meshspawntransform_rotation false false)
    (set `self.IsRagdolled` false)))

(event `self.ForceImpulseMovement`
  (params (Impulse :type "Vector Structure"))
  ;[1 1 1] Ragdoll Physics
  (`PrimitiveComponent.AddImpulse` (`self.Mesh`) Impulse "None" false))

(event `self.PlaySoundAttached`
  (params (Sound :type "SoundBase Object Reference"))
  ;[1 1 1] Actor Sound
  (`GameplayStatics.SpawnSoundAttached` Sound (`self.Mesh`) "None" (0.0 0.0 0.0) (struct) "KeepRelativeOffset" false 1.0 1.0 0.0 null null)
  (`PawnNoiseEmitterComponent.MakeNoise` (`self.PawnNoiseEmitter`) self 1.0 (`self.K2_GetActorLocation`)))

(event `self.PlaySoundAtLocation`
  (params (SoundBase :type "SoundBase Object Reference"))
  (bind _returnvalue (`SceneComponent.K2_GetComponentLocation` (`self.Mesh`)))
  ;[1 1 1] Actor Sound
  (`GameplayStatics.PlaySoundAtLocation` SoundBase _returnvalue (struct) 1.0 1.0 0.0 null null null null)
  (`PawnNoiseEmitterComponent.MakeNoise` (`self.PawnNoiseEmitter`) self 1.0 _returnvalue))

(event `EnableMovement`
  (`CharacterMovementComponent.SetMovementMode` (`self.CharacterMovement`) "MOVE_Walking" 0))

(fn `AllowDamageCheck`
  (params (TargetActor :type "Actor Object Reference"))
  (returns (CanDamage :type Boolean))
  (if (and (!= TargetActor self) (`KismetSystemLibrary.DoesImplementInterface` TargetActor "/Game/Blueprints/Interfaces/BPI_Combat.BPI_Combat_C"))
    (if (== TargetActor (`self.LastAttackedTarget`))
      (return false)
      (else
        (set `self.LastAttackedTarget` TargetActor)
        (return true)))
    (else
      (return false))))

(fn `CalculateDamage`
  (params (DamageAmount :type "Float (double-precision)"))
  (set `self.CurrentHealth` (`KismetMathLibrary.FClamp` (- (`self.CurrentHealth`) DamageAmount) 0.0 (`self.MaxHealth`)))
  (if (>= DamageAmount 10.0)
    (`self.TakeDamageEffects`)))

(fn `TakeDamageEffects`
  (`NiagaraFunctionLibrary.SpawnSystemAtLocation` "/Game/Particles/PS_Blood_Burst.PS_Blood_Burst" (`SceneComponent.K2_GetComponentLocation` (`self.Mesh`)))
  (`self.PlaySoundAttached` (`self.DamageTakenSound`)))

(fn `UserConstructionScript`)