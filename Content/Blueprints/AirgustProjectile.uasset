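; An air gust projectile that ragdolls and scatters the physics-interface actors it overlaps, excluding the player character.
; Initialize sets its speed and scales its lifespan by the ratio of that speed to the maximum.
; Tick sweeps it forward by Speed each frame, without delta-time scaling.
; On sphere overlap, it sends interface messages for a timed ragdoll and a speed-scaled impulse in a random, wide forward-centred cone.
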(event `Initialize`
  (params (Speed :type "Float (double-precision)") (MaxSpeed :type "Float (double-precision)"))
  (bind _output_get (set `self.Speed` Speed))
  (`self.SetLifeSpan` (+ (* (/ _output_get MaxSpeed) (`self.MaxLifetime`)) 0.1)))

(event `self.ReceiveTick`
  (params (DeltaSeconds :type "Float (single-precision)"))
  (bind (_returnvalue_location _returnvalue_rotation _returnvalue_scale) (`KismetMathLibrary.BreakTransform` (`self.GetTransform`)))
  (`self.K2_SetActorTransform` (`KismetMathLibrary.MakeTransform` (+ (`self.K2_GetActorLocation`) (* (`self.GetActorForwardVector`) (`self.Speed`))) _returnvalue_rotation _returnvalue_scale) true))

(event `self.SphereTrigger.OnComponentBeginOverlap`
  (params (OverlappedComponent :type "PrimitiveComponent Object Reference") (OtherActor :type "Actor Object Reference") (OtherComp :type "PrimitiveComponent Object Reference") (OtherBodyIndex :type Integer) (bFromSweep :type Boolean) (SweepResult :type "HitResult Structure (by ref)"))
  (if (and (`KismetSystemLibrary.DoesImplementInterface` OtherActor "/Game/Blueprints/Interfaces/Physics.Physics_C") (!= (`GameplayStatics.GetObjectClass` OtherActor) "/Game/Blueprints/BP_PlayerCharacter.BP_PlayerCharacter_C"))
    (message `/Game/Blueprints/Interfaces/Physics.ToggleRagdoll` OtherActor true 3.0)
    (message `/Game/Blueprints/Interfaces/Physics.ForceImpulseMovement` OtherActor (* (`KismetMathLibrary.RandomUnitVectorInConeInDegrees` (`self.GetActorForwardVector`) 120.0) (* (+ (`self.Speed`) 1.0) 20.0)))))

(fn `UserConstructionScript`)