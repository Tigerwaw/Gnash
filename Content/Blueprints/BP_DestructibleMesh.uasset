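; BP_DestructibleMesh is a destructible barrel actor that breaks through Chaos physics and can be pushed by impulses.
; On break, it plays a quiet wood-breaking sound, emits noise through a PawnNoiseEmitter, and sets a short lifespan so it cleans itself up.
; ForceImpulseMovement applies a caller-supplied impulse to the barrel, while TakeDamage applies a fixed large impulse regardless of the hit.
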(event `self.Barrel_Destructible.OnChaosBreakEvent`
  (params (BreakEvent :type "ChaosBreakEvent Structure (by ref)"))
  (`GameplayStatics.PlaySoundAtLocation` "/Game/Sounds/SFX/Impacts/WoodBreaking_Cue.WoodBreaking_Cue" (`SceneComponent.K2_GetComponentLocation` (`self.Barrel_Destructible`)) (struct) 0.1 1.0 0.0 "/Game/Sounds/AttenuationPresets/Attenuation_Quiet.Attenuation_Quiet" null null null)
  (`PawnNoiseEmitterComponent.MakeNoise` (`self.PawnNoiseEmitter`) self 1.0 (`SceneComponent.K2_GetComponentLocation` (`self.Barrel_Destructible`)))
  (`self.SetLifeSpan` 15.0))

(event `/Game/Blueprints/Interfaces/BPI_Physics.ForceImpulseMovement`
  (params (Impulse :type "Vector Structure"))
  (`PrimitiveComponent.AddImpulse` (`self.Barrel_Destructible`) Impulse "None" false))

(event `/Game/Blueprints/Interfaces/BPI_Combat.TakeDamage`
  (params (DamageAmount :type "Float (double-precision)") (Attacker :type "Actor Object Reference"))
  (`PrimitiveComponent.AddImpulse` (`self.Barrel_Destructible`) (100000.0 100000.0 10000.0) "None" false))

(fn `UserConstructionScript`)