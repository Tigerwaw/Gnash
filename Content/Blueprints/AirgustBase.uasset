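; AirgustBase is an air gust actor that travels forward and grows, with no hit response in its graphs.
; Initialize stores the speed and sets its lifespan from MaxLifetime.
; Each Tick lerps the current scale toward MaxSize by time alive over GrowTime, compounding the growth.
; It also makes a swept move along its forward vector by Speed per frame, unscaled by delta time.
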(event `Initialize`
  (params (Speed :type "Float (double-precision)"))
  (set `self.Speed` Speed)
  (`self.SetLifeSpan` (`self.MaxLifetime`)))

(event `self.ReceiveTick`
  (params (DeltaSeconds :type "Float (single-precision)"))
  (set `self.CurrentTimeAlive` (+ DeltaSeconds (`self.CurrentTimeAlive`)))
  (`|ExecutionSequence`
    (:`then_0`
      (`self.SetActorRelativeScale3D` (`KismetMathLibrary.VLerp` (`self.GetActorRelativeScale3D`) (`self.MaxSize`) (/ (`self.CurrentTimeAlive`) (`self.GrowTime`)))))
    (:`then_1`
      (`self.K2_SetActorLocation` (+ (`self.K2_GetActorLocation`) (* (`self.GetActorForwardVector`) (`self.Speed`))) true))))

(fn `UserConstructionScript`)