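; Gun projectile actor with a limited lifetime that damages combat actors and can ricochet once off other surfaces.
; On hit, BPI_Combat actors receive randomly varied damage and a flesh-impact sound via interface messages, then the projectile is destroyed.
; Other hits compare surface normal to velocity with a dot product to either destroy it or flag a ricochet with sound.
; Hitting an AirgustProjectile only prints a deflection message.
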(event `self.ReceiveBeginPlay`
  (`self.SetLifeSpan` (`self.MaxLifetime`)))

(event `self.Sphere.OnComponentHit`
  (params (HitComponent :type "PrimitiveComponent Object Reference") (OtherActor :type "Actor Object Reference") (OtherComp :type "PrimitiveComponent Object Reference") (NormalImpulse :type "Vector Structure") (Hit :type "HitResult Structure (by ref)"))
  (if (`KismetSystemLibrary.DoesImplementInterface` OtherActor "/Game/Blueprints/Interfaces/BPI_Combat.BPI_Combat_C")
    (`self.DealDamage` OtherActor)
    (elif (== (`GameplayStatics.GetObjectClass` OtherActor) "/Game/Blueprints/PlayerCharacter/AirgustProjectile.AirgustProjectile_C")
      (`KismetSystemLibrary.PrintString` "Bullet Deflected")
      (elif (or (> (`KismetMathLibrary.Dot_VectorVector` Hit_Normal (`KismetMathLibrary.Normal` (`SceneComponent.GetComponentVelocity` (`self.Sphere`)))) 0.75) (`self.HasRicocheted`))
        (`self.EnvironmentImpact`)
        (else
          (`self.Ricochet` Hit_Location))))))

(event `DealDamage`
  (params (OtherActor :type "Actor Object Reference"))
  (bind _damage (`self.CalculateDamage`))
  (message `/Game/Blueprints/Interfaces/BPI_Combat.TakeDamage` OtherActor _damage (`self.GetInstigator`))
  (message `/Game/Blueprints/Interfaces/BPI_ActorSoundEffects.PlaySoundAtLocation` OtherActor "/Game/Sounds/SFX/Impacts/BulletFleshImpact_Cue.BulletFleshImpact_Cue")
  (`self.K2_DestroyActor`))

(event `EnvironmentImpact`
  (`self.K2_DestroyActor`))

(event `Ricochet`
  (params (HitLocation :type "Vector Structure"))
  (`GameplayStatics.PlaySoundAtLocation` "/Game/Sounds/SFX/Gun/WallRicochet_Cue.WallRicochet_Cue" HitLocation (struct) 1.0 1.0 0.0 null null null null)
  (set `self.HasRicocheted` true))

(fn `CalculateDamage`
  (returns (Damage :type "Float (double-precision)"))
  (return (`/Game/Blueprints/FL_Misc.RandomVarianceFloat` (`self.BaseDamage`) (`self.DamageVariance`))))

(fn `UserConstructionScript`)